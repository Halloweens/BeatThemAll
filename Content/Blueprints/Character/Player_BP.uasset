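; Player character Blueprint handling HUD, footsteps, weapon pickup, pausing and death.
; After a delayed intro, it destroys tagged intro cameras, activates its own camera and shows the HP bar.
; Foot triggers trace downward to spawn footprint decals and play surface-selected sound, with only Sand assigned.
; Capsule overlaps call weapon pickup, M opens a cached pause menu, and Tick loads the death level when health runs out.
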(event `self.ReceiveBeginPlay`
  (bind _returnvalue (`|CreateWidget` "/Game/Blueprints/HPBar/PlayerHPBar.PlayerHPBar_C"))
  (`KismetSystemLibrary.Delay` 11.0)
  (`self.DoIntro`)
  (`ActorComponent.Activate` (`self.Camera`) true)
  (`UserWidget.AddToViewport` _returnvalue 0))

(event `LeftFeet`
  (`self.footPrint` (`self.leftfoot`))
  (`self.Footsound` (`self.rightfoot`) :!label _label))

(event `rightFeet`
  (`self.footPrint` (`self.rightfoot`))
  (goto _label))

(event `self.ReceiveTick`
  (params (DeltaSeconds :type "Float (single-precision)"))
  (if (<= (`self.CurrentHp`) 0.0)
    (`GameplayStatics.OpenLevel` "DeathScreen")))

(event `Key|M`
  (params (Key :type "Key Structure" :default "AnyKey"))
  (bind _returnvalue (`GameplayStatics.GetPlayerController` 0))
  (bind _pausemenu (`self.PauseMenu`))
  (:`Pressed`
    (`/Engine/EditorBlueprintResources/StandardMacros.IsValid` _pausemenu
      (:`Is Valid`
        _)
      (:`Is Not Valid`
        (bind _returnvalue_2 (`|CreateWidget` "/Game/Gui/PauseMenu.PauseMenu_C"))
        (set `self.PauseMenu` _returnvalue_2)))
    (`WidgetBlueprintLibrary.SetInputMode_UIOnlyEx` _returnvalue _pausemenu)
    (`UserWidget.AddToViewport` _pausemenu 0)
    (set `PlayerController.bShowMouseCursor` true _returnvalue)
    (`GameplayStatics.SetGamePaused` true)))

(event `self.CapsuleComponent.OnComponentBeginOverlap`
  (params (OverlappedComponent :type "PrimitiveComponent Object Reference") (OtherActor :type "Actor Object Reference") (OtherComp :type "PrimitiveComponent Object Reference") (OtherBodyIndex :type Integer) (bFromSweep :type Boolean) (SweepResult :type "HitResult Structure (by ref)"))
  (`self.pickUpWeapon` OtherComp))

(fn `DoIntro`
  (bind _outactors (`GameplayStatics.GetAllActorsOfClass` "/Game/Blueprints/IntroSequenceCamera_Blueprint.IntroSequenceCamera_Blueprint_C"))
  (for _array_element _outactors
    (bind _asintro_sequence_camera_blueprint (cast `/Game/Blueprints/IntroSequenceCamera_Blueprint` _array_element))
    (if (`self.ActorHasTag` _asintro_sequence_camera_blueprint "Intro")
      (`self.K2_DestroyActor` _asintro_sequence_camera_blueprint))))

(fn `footPrint`
  (params (Target :type "SceneComponent Object Reference"))
  (bind _returnvalue (`SceneComponent.K2_GetComponentLocation` Target))
  (bind _outhit (`KismetSystemLibrary.LineTraceSingle` (+ _returnvalue (0.0 0.0 20.0)) (- _returnvalue (0.0 0.0 20.0)) "TraceTypeQuery1"))
  (`GameplayStatics.SpawnDecalAtLocation` "/Game/Other/FootPrint.FootPrint" (20.0 20.0 20.0) (`.Location` (`GameplayStatics.BreakHitResult` _outhit)) (`KismetMathLibrary.MakeRotator` -90.0 90.0 (.yaw (`SceneComponent.K2_GetComponentRotation` Target))))
  (return))

(fn `Footsound`
  (params (self2 :type "ActorComponent Object Reference"))
  (bind _returnvalue (`self.K2_GetActorLocation` (`ActorComponent.GetOwner` self2)))
  (bind (_outhit _returnvalue_2) (`KismetSystemLibrary.LineTraceSingle` (+ _returnvalue (0.0 0.0 330.0)) (- _returnvalue (0.0 0.0 300.0)) "TraceTypeQuery1"))
  (if _returnvalue_2
    (`GameplayStatics.PlaySoundAtLocation` (select `EPhysicalSurface` (`GameplayStatics.GetSurfaceType` _outhit) :`SurfaceType1` "/Game/Sounds/Ambiant/Walk.Walk" :!type "SoundBase Object Reference") (`.Location` (`GameplayStatics.BreakHitResult` _outhit))))
  (return))

(fn `getBox`
  (returns (collisionbox :type "BoxComponent Object Reference"))
  (return (`self.Box`)))

(fn `LeftFootTrigger`
  (`self.LeftFeet`))

(fn `RightFootTrigger`
  (`self.rightFeet`))

(fn `UserConstructionScript`
  (set `self.WeaponCollider` (`self.Box`))
  (set `self.WeapondWrap` (`self.weaponWrapper`))
  (set `self.shieldWrap` (`self.ShieldWrapper`))
  (set `self.characterBody` (`self.CapsuleComponent`))
  (set `self.Blood` "/Game/Environment/Effects/particles/Blood.Blood"))