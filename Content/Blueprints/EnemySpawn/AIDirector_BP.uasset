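; AI director Blueprint that tracks enemy deaths and opens the WinningScreen level once the enemy count runs out.
; Every Tick it gathers all Enemy_BP actors and passes them to the WinScreen function.
; WinScreen decrements NumberEnemy for each enemy at zero HP or below, using that enemy's Verifications flag to count it only once.
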(event `self.ReceiveTick`
  (params (DeltaSeconds :type "Float (single-precision)"))
  (bind _outactors (`GameplayStatics.GetAllActorsOfClass` "/Game/Blueprints/Character/Enemy_BP.Enemy_BP_C"))
  (`self.WinScreen` _outactors))

(fn `UserConstructionScript`)

(fn `WinScreen`
  (params (Object :type "Array of Enemy Object Reference"))
  (for _array_element Object
    (bind _asenemy (cast `Enemy` _array_element))
    (if (<= (`MyCharacter.CurrentHp` _asenemy) 0.0)
      (if (not (`MyCharacter.verifications` _asenemy))
        (set `MyCharacter.verifications` true _asenemy)
        (bind _output_get (set `self.numberEnemy` (- (`self.numberEnemy`) 1.0)))
        (if (<= _output_get 0.0)
          (`GameplayStatics.OpenLevel` "WinningScreen"))))))